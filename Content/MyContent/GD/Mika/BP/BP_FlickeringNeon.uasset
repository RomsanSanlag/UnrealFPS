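; BP_FlickeringNeon is a rect light actor that imitates a faulty neon light.
; BeginPlay plays a neon buzz sound at the actor's location and starts the Flicker loop.
; Flicker waits a random several seconds, blinks the light off briefly, pauses shortly, blinks again, then calls itself to repeat indefinitely.
; TurnOff and TurnOn toggle the RectLightComponent's visibility, with randomized delays keeping the pattern irregular.
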(event Custom|Flicker
  (Utilities|FlowControl|Delay (Math|Random|RandomFloatinRange 5.0 15.0))
  (CallFunction|TurnOff)
  (Utilities|FlowControl|Delay (Math|Random|RandomFloatinRange 0.1 0.15))
  (CallFunction|Turnon)
  (Utilities|FlowControl|Delay (Math|Random|RandomFloatinRange 0.25 2.0))
  (CallFunction|TurnOff)
  (Utilities|FlowControl|Delay (Math|Random|RandomFloatinRange 0.1 0.15))
  (CallFunction|Turnon)
  (CallFunction|Flicker))

(event Custom|Turn%20On
  (Rendering|SetVisibility (Variables|Default|GetRectLightComponent) true false))

(event Custom|Turn%20Off
  (Rendering|SetVisibility (Variables|Default|GetRectLightComponent) false false))

(event EventBeginPlay
  (Audio|PlaySoundatLocation "/Game/MyContent/GD/Mika/Sounds/Sound_NeonBuzz_Cue.Sound_NeonBuzz_Cue" (Transformation|GetActorLocation) "0, 0, 0" 1.0 1.0 0.0 0 0 0 0)
  (Utilities|FlowControl|Delay (Math|Random|RandomFloatinRange 5.0 15.0))
  (CallFunction|TurnOff)
  (Utilities|FlowControl|Delay (Math|Random|RandomFloatinRange 0.1 0.15))
  (CallFunction|Turnon)
  (Utilities|FlowControl|Delay (Math|Random|RandomFloatinRange 0.25 2.0))
  (CallFunction|TurnOff)
  (Utilities|FlowControl|Delay (Math|Random|RandomFloatinRange 0.1 0.15))
  (CallFunction|Turnon)
  (CallFunction|Flicker))

(fn ConstructionScript)