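; BP_GridChecker is the controller for a pressure plate grid puzzle that opens a door.
; Check sends OpenMessage to the Door when the Good count equals the Grid array's length.
; ResetGrid zeroes the count, resets every BP_PressurePlate in the level and briefly raises the Sphere material's Intensity through a Delay placed inside the loop.
; EventWrong calls Wrong on every plate.
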(event Custom|EventWrong
  (bind _outactors (Actor|GetAllActorsOfClass "/Game/MyContent/GP/BPVictor/BP_PressurePlate.BP_PressurePlate_C"))
  (for _array_element _outactors
    (Default|Wrong _array_element)))

(event Custom|Check
  (if (== (Variables|Default|GetGood) (Utilities|Array|Length (Variables|Default|GetGrid)))
    (Class|IOpenable|Open(Message) (Variables|Default|GetDoor))))

(event Custom|ResetGrid
  (Variables|Default|SetGood 0)
  (bind _outactors (Actor|GetAllActorsOfClass "/Game/MyContent/GP/BPVictor/BP_PressurePlate.BP_PressurePlate_C"))
  (for _array_element _outactors
    (Default|Reset _array_element)
    (Rendering|Material|SetScalarParameterValueonMaterials (Variables|Default|GetSphere) "Intensity" 2e+01)
    (Utilities|FlowControl|Delay 1.5)
    (Rendering|Material|SetScalarParameterValueonMaterials (Variables|Default|GetSphere) "Intensity" 4.0)))

(fn ConstructionScript)