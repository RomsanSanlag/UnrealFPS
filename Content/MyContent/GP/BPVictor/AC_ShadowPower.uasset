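; Actor component that gives the player character two shadow powers: an aimed teleport and a projectile shot.
; Power one traces from the camera to position a BP_TPPortal Niagara marker, then on completion teleports the character to the hit's XY, keeping its height.
; Power two launches a BP_Projectile along the control rotation, gated by CanShoot, which is not reset here.
; SetPortal keeps at most two portals, removing the oldest; projectile path prediction is unconnected.
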(event EventPowerTwoCompleted
  (bind _characterref (Variables|Default|GetCharacterRef))
  (bind _camera (Variables|/Game/MyContent/GP/Game/BP_Character.BP_Character_C|GetCamera _characterref))
  (if (Variables|Default|GetCanShoot)
    (Variables|Default|SetCanShoot false)
    (bind _returnvalue (Game|SpawnActorfromClass "/Game/MyContent/GP/BPVictor/BP_Projectile.BP_Projectile_C" (Math|Transform|MakeTransform (+ (Transformation|GetWorldLocation _camera) (* (Math|Vector|GetForwardVector _camera) (Math|Float|MakeLiteralFloat 1e+02))) "0, 0, 0" "1.000000,1.000000,1.000000") "Undefined" 0 0))
    (Physics|SetPhysicsLinearVelocity (Variables|/Game/MyContent/GP/BPVictor/BP_Projectile.BP_Projectile_C|GetSphere _returnvalue) (* (Math|Vector|GetForwardVector (Pawn|GetControlRotation (Variables|Default|GetCharacterRef) :!class /Script/Engine.Pawn)) (Math|Float|MakeLiteralFloat 3e+03)) false "None")))

(event EventPowerTwoTriggered)

(event EventBeginPlay
  (bind _asbp_character (Utilities|Casting|CastToBP_Character (Game|GetPlayerCharacter 0)))
  (Variables|Default|SetCharacterRef _asbp_character))

(event EventPowerOneTriggered
  (bind _characterref (Variables|Default|GetCharacterRef))
  (bind _camera (Variables|/Game/MyContent/GP/Game/BP_Character.BP_Character_C|GetCamera _characterref))
  (bind _returnvalue (Transformation|GetWorldLocation _camera))
  (bind (_outhit _returnvalue_2) (Collision|LineTraceByChannel _returnvalue (+ _returnvalue (* (Math|Vector|GetForwardVector _camera) (Variables|Default|GetTpRange))) "TraceTypeQuery4" false 0 "None"))
  (Transformation|SetActorLocation (stale EventPowerOneStarted _returnvalue) (Math|Vector|MakeVector (.x (.ImpactPoint (Collision|BreakHitResult _outhit))) (.y (.ImpactPoint (Collision|BreakHitResult _outhit))) (+ (.z (.ImpactPoint (Collision|BreakHitResult _outhit))) 1e+01)) false true))

(event EventPowerOneCompleted
  (if (stale EventPowerOneTriggered _returnvalue_2)
    (Transformation|SetActorLocation (Variables|Default|GetCharacterRef) (Math|Vector|MakeVector (.x (.ImpactPoint (Collision|BreakHitResult (stale EventPowerOneTriggered _outhit)))) (.y (.ImpactPoint (Collision|BreakHitResult (stale EventPowerOneTriggered _outhit)))) (+ 0.0 (.z (Transformation|GetActorLocation (Variables|Default|GetCharacterRef))))) false false)
    (Rendering|SetVisibility (Variables|/Game/MyContent/GP/BPVictor/BP_TPPortal.BP_TPPortal_C|GetNiagara (stale EventPowerOneStarted _returnvalue)) false false)))

(event EventPowerOneStarted
  (bind _returnvalue (Actor|GetActorOfClass "/Game/MyContent/GP/BPVictor/BP_TPPortal.BP_TPPortal_C"))
  (Rendering|SetVisibility (Variables|/Game/MyContent/GP/BPVictor/BP_TPPortal.BP_TPPortal_C|GetNiagara _returnvalue) true false))

(fn SetPortal
  (params (Portal :type BP%20Portal%20Object%20Reference))
  (if (and (Utilities|IsValid (Variables|Default|GetPortal1)) (Utilities|IsValid (Variables|Default|GetPortal2)))
    (Default|Remove (Variables|Default|GetPortal1))
    (Variables|Default|SetPortal1 (Variables|Default|GetPortal2))
    (Variables|Default|SetPortal2 Portal)
    (elif (Utilities|IsValid (Variables|Default|GetPortal1))
      (if (not (Utilities|IsValid (Variables|Default|GetPortal2)))
        (Variables|Default|SetPortal2 Portal))
      (else
        (Variables|Default|SetPortal1 Portal)))))