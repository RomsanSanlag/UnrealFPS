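; BP_ObjectsDeathZone is a trigger volume that sends objects entering it back through their reset logic.
; On Box overlap, it acts only on actors that have an AC_Reset component.
; It zeroes the linear velocity of all physics bodies on the actor's primitive component, then calls ResetPosition on AC_Reset.
; An unconnected variant that checks the primitive component first never runs.
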(event OnComponentBeginOverlap(Box)
  (params (OverlappedComponent :type Primitive%20Component%20Object%20Reference) (OtherActor :type Actor%20Object%20Reference) (OtherComp :type Primitive%20Component%20Object%20Reference) (OtherBodyIndex :type Integer) (bFromSweep :type Boolean) (SweepResult :type Hit%20Result%20Structure%20%28by%20ref%29))
  (bind _returnvalue (Actor|GetComponentbyClass OtherActor "/Game/MyContent/GP/BPVictor/AC_Reset.AC_Reset_C"))
  (Utilities|IsValid _returnvalue
    (:Is%20Valid
      (Class|PrimitiveComponent|SetAllPhysicsLinearVelocity (Actor|GetComponentbyClass OtherActor "/Script/Engine.PrimitiveComponent") "0, 0, 0" false)
      (Default|ResetPosition _returnvalue))))

(event Collision|EventActorBeginOverlap
  (params (OtherActor :type Actor%20Object%20Reference)))

(fn ConstructionScript)