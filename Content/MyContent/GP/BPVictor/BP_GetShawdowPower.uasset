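; Trigger actor that registers the shadow power with the player, firing only once.
; The first box overlap sets a touched flag and casts player controller 0 to PC_Character.
; If the overlapping actor has an AC_ShadowPower component, that component is added to the controller's Powers array and every entry in Change receives SwitchMessage.
; The flag is set before that check, so any first overlap consumes the trigger.
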(event OnComponentBeginOverlap(Box)
  (params (OverlappedComponent :type Primitive%20Component%20Object%20Reference) (OtherActor :type Actor%20Object%20Reference) (OtherComp :type Primitive%20Component%20Object%20Reference) (OtherBodyIndex :type Integer) (bFromSweep :type Boolean) (SweepResult :type Hit%20Result%20Structure%20%28by%20ref%29))
  (bind _returnvalue (Actor|GetComponentbyClass OtherActor "/Game/MyContent/GP/BPVictor/AC_ShadowPower.AC_ShadowPower_C"))
  (if (not (Variables|Default|GetWasTouched))
    (Variables|Default|SetWasTouched true)
    (bind _aspc_character (Utilities|Casting|CastToPC_Character (Game|GetPlayerController 0)))
    (if (Utilities|IsValid _returnvalue)
      (Utilities|Array|Add (Variables|/Game/MyContent/GP/Game/PC_Character.PC_Character_C|GetPowers _aspc_character) _returnvalue)
      (for _array_element (Variables|Default|GetChange)
        (Class|IChangeRoom|Switch(Message) _array_element)))))

(fn ConstructionScript)