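; BP_GridSpawner builds and manages a grid of BP_MineDetector actors for a mine path puzzle.
; MakeGrid clears old detectors, then spawns new ones spaced by Offset, attaches them and gives each a reference back to the spawner.
; CheckGrid compares CountPath with GoodPathNUm, with only a placeholder print on a match.
; Reset zeroes CountPath and resets every mine.
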(event Custom|Make%20Grid
  (bind _self self)
  (bind _gridsize (Variables|Default|GetGridSize))
  (bind _offset (Variables|Default|GetOffset))
  (CallFunction|Clear)
  (for _index (range 1 (Math|Float|Truncate (.x _gridsize)))
    (for _index_2 (range 1 (Math|Float|Truncate (.y _gridsize)))
      (bind _returnvalue (Game|SpawnActorfromClass "/Game/MyContent/GP/BPVictor/BP_MineDetector.BP_MineDetector_C" (Math|Transform|MakeTransform (+ (Math|Vector|MakeVector (* _index _offset) (* _index_2 _offset) 0.0) (Transformation|GetActorLocation)) "0, 0, 0" "1.000000,1.000000,1.000000") "Undefined" 0 0))
      (Utilities|Array|Add (Variables|Default|GetMines) _returnvalue)
      (Transformation|AttachActorToActor _returnvalue _self "None" "KeepWorld" "KeepWorld" "KeepWorld" true)
      (Variables|/Game/MyContent/GP/BPVictor/BP_MineDetector.BP_MineDetector_C|SetGridSpawnerRef _returnvalue _self))))

(event Custom|Clear
  (bind _mines (Variables|Default|GetMines))
  (for _array_element _mines
    (Actor|DestroyActor _array_element))
  (Utilities|Array|Clear _mines))

(event Custom|Reset
  (Development|PrintString "Reseted")
  (Variables|Default|SetCountPath 0)
  (for _array_element (Variables|Default|GetMines)
    (Default|ResetMine _array_element)))

(event Custom|CheckGrid
  (Development|PrintString (Utilities|String|ToString(Integer) (Variables|Default|GetGoodPathNUm)))
  (Development|PrintString (Utilities|String|ToString(Integer) (Variables|Default|GetCountPath)))
  (if (== (Variables|Default|GetGoodPathNUm) (Variables|Default|GetCountPath))
    (Development|PrintString "Do Something")))

(event EventBeginPlay
  (Variables|Default|SetCountPath 0))

(fn ConstructionScript)