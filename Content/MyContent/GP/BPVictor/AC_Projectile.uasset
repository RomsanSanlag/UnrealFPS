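; Actor component that predicts and fires projectiles from the player character's camera.
; BeginPlay caches the BP_Character, whose camera location and control rotation set launch origin and direction.
; CE_ShootProjectile spawns BP_Projectile and sets its sphere's physics velocity.
; CE_DrawTrajectorie predicts the path by trace channel at the same hardcoded speed, but its loop over path points is empty.
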(event Custom|CE_DrawTrajectorie
  (bind _characterref (Variables|Default|GetCharacterRef))
  (bind _outpathpositions (Class|GameplayStatics|BlueprintPredictProjectilePathbyTraceChannel (Transformation|GetWorldLocation (Variables|/Game/MyContent/GP/Game/BP_Character.BP_Character_C|GetCamera _characterref)) (* (Math|Vector|GetForwardVector (Pawn|GetControlRotation _characterref :!class /Script/Engine.Pawn)) (Math|Float|MakeLiteralFloat 3e+03)) true 0.0 "ECC_GameTraceChannel3" false (Utilities|Array|MakeArray _characterref) "None"))
  (for _array_element _outpathpositions
    _))

(event Custom|CE_ShootProjectile
  (bind _characterref (Variables|Default|GetCharacterRef))
  (bind _returnvalue (Game|SpawnActorfromClass "/Game/MyContent/GP/BPVictor/BP_Projectile.BP_Projectile_C" (Math|Transform|MakeTransform (Transformation|GetWorldLocation (Variables|/Game/MyContent/GP/Game/BP_Character.BP_Character_C|GetCamera _characterref)) "0, 0, 0" "1.000000,1.000000,1.000000") "Undefined" 0 0))
  (Physics|SetPhysicsLinearVelocity (Variables|/Game/MyContent/GP/BPVictor/BP_Projectile.BP_Projectile_C|GetSphere _returnvalue) (* (Math|Vector|GetForwardVector (Pawn|GetControlRotation _characterref :!class /Script/Engine.Pawn)) (Math|Float|MakeLiteralFloat 3e+03)) false "None"))

(event EventBeginPlay
  (bind _asbp_character (Utilities|Casting|CastToBP_Character (Game|GetPlayerCharacter 0)))
  (Variables|Default|SetCharacterRef _asbp_character))