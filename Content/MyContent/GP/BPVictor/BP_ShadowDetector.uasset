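; BP_ShadowDetector is a spotlight hazard that kills and respawns the player character when it is caught in direct view of the light.
; Switch turns on detection and the light.
; While the player overlaps the actor, Tick line-traces from the spotlight to the player, so blocking geometry provides cover.
; A hit triggers an animated death screen, then after a delay teleports the player to RespawnPoint and removes the screen.
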(event Custom|CE_Death
  (bind _returnvalue (UserInterface|CreateWidget "/Game/MyContent/GP/UMG/W_DeathScreen.W_DeathScreen_C"))
  (UserInterface|Viewport|AddtoViewport _returnvalue 0)
  (UserInterface|Animation|PlayAnimation _returnvalue (Variables|/Game/MyContent/GP/UMG/W_DeathScreen.W_DeathScreen_C|GetScreenAnimation _returnvalue) 0.0 1 "Forward" 1.0 false)
  (Utilities|FlowControl|Delay 2.0)
  (Transformation|SetActorLocation (Variables|Default|GetAs%20BP%20Character) (Transformation|GetActorLocation (Variables|Default|GetRespawnPoint)) false true)
  (bind _foundwidgets (Widget|GetAllWidgetsOfClass "/Game/MyContent/GP/UMG/W_DeathScreen.W_DeathScreen_C" true))
  (Widget|RemovefromParent _foundwidgets))

(event EventSwitch
  (Variables|Default|SetCanDetect true)
  (Rendering|SetVisibility (Variables|Default|GetSpotLight) true false))

(event EventBeginPlay
  (bind _asbp_character (Utilities|Casting|CastToBP_Character (Game|GetPlayerCharacter 0)))
  (Variables|Default|SetAs%20BP%20Character _asbp_character))

(event Collision|EventActorBeginOverlap
  (params (OtherActor :type Actor%20Object%20Reference))
  (Utilities|Casting|CastToBP_Character OtherActor)
  (Variables|Default|SetOverlap true))

(event Collision|EventActorEndOverlap
  (params (OtherActor :type Actor%20Object%20Reference))
  (Utilities|Casting|CastToBP_Character OtherActor)
  (Variables|Default|SetOverlap false))

(event EventTick
  (params (DeltaSeconds :type Float%20%28single-precision%29))
  (if (Variables|Default|GetCanDetect)
    (if (Variables|Default|GetOverlap)
      (bind _outhit (Collision|LineTraceByChannel (Transformation|GetWorldLocation (Variables|Default|GetSpotLight)) (Transformation|GetActorLocation (Game|GetPlayerCharacter 0)) "TraceTypeQuery1" false 0 "None"))
      (Utilities|Casting|CastToBP_Character (.hitactor _outhit))
      (CallFunction|CEDeath))))

(fn ConstructionScript)