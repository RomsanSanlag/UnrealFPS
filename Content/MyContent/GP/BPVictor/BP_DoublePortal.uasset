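; BP_DoublePortal polices the BP_Portal actors in the level, calling Remove on a selected portal.
; Each Tick it gathers all portals and acts only when one or two exist.
; It scans them for the greatest GetLifeSpan value and calls Remove on the portal at the stored index.
; The Lifetime and Index variables are never reset, so earlier maxima carry into later ticks.
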(event EventTick
  (params (DeltaSeconds :type Float%20%28single-precision%29))
  (bind _outactors (Actor|GetAllActorsOfClass "/Game/MyContent/GP/BPVictor/BP_Portal.BP_Portal_C"))
  (if (> (Utilities|Array|Length _outactors) 0)
    (if (< (Utilities|Array|Length _outactors) 3)
      (for (_array_element _array_index) _outactors
        (if (> (Actor|GetLifeSpan _array_element) (Variables|Default|GetLifetime))
          (Variables|Default|SetLifetime (Actor|GetLifeSpan _array_element))
          (Variables|Default|SetIndex _array_index)))
      (Default|Remove (Utilities|Array|Get(acopy) _outactors (Variables|Default|GetIndex))))))

(fn ConstructionScript)