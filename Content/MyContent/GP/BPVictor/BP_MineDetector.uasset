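; BP_MineDetector is a grid tile in a path puzzle that is either part of the good path or a mine.
; Its Path event toggles that state, swapping the cube material and adjusting the good-path total on GridSpawnerRef.
; The first BP_Character overlap either advances the spawner's path count and runs CheckGrid, or resets the spawner on a wrong tile.
; ResetMine clears the touched flag.
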(event OnComponentBeginOverlap(Box)
  (params (OverlappedComponent :type Primitive%20Component%20Object%20Reference) (OtherActor :type Actor%20Object%20Reference) (OtherComp :type Primitive%20Component%20Object%20Reference) (OtherBodyIndex :type Integer) (bFromSweep :type Boolean) (SweepResult :type Hit%20Result%20Structure%20%28by%20ref%29))
  (bind _gridspawnerref (Variables|Default|GetGridSpawnerRef))
  (Utilities|Casting|CastToBP_Character OtherActor)
  (if (not (Variables|Default|GetWasTouched))
    (Variables|Default|SetWasTouched true)
    (if (Variables|Default|GetGoodPath)
      (Math|Integer|IncrementInt (Variables|/Game/MyContent/GP/BPVictor/BP_GridSpawner.BP_GridSpawner_C|GetCountPath _gridspawnerref)
        (:%20%20
          (Default|CheckGrid _gridspawnerref)))
      (else
        (Default|Reset _gridspawnerref)))))

(event Custom|Path
  (bind _cube (Variables|Default|GetCube))
  (Utilities|FlowControl|FlipFlop
    (:A
      (Variables|Default|SetGoodPath true)
      (Rendering|Material|SetMaterial _cube 0 "/Game/MyContent/GP/Materials/M_Blue.M_Blue")
      (Math|Integer|IncrementInt (Variables|/Game/MyContent/GP/BPVictor/BP_GridSpawner.BP_GridSpawner_C|GetGoodPathNUm (Variables|Default|GetGridSpawnerRef))))
    (:B
      (Variables|Default|SetGoodPath false)
      (Rendering|Material|SetMaterial _cube 0 "/Game/StarterContent/Materials/M_Basic_Wall.M_Basic_Wall")
      (Math|Integer|DecrementInt (Variables|/Game/MyContent/GP/BPVictor/BP_GridSpawner.BP_GridSpawner_C|GetGoodPathNUm (Variables|Default|GetGridSpawnerRef))))))

(event Custom|ResetMine
  (Variables|Default|SetWasTouched false)
  (if (Variables|Default|GetWasTouched)
    _))

(fn ConstructionScript)