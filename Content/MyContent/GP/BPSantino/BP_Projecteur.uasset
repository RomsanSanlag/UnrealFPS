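; BP_Projecteur is a two-slot projector puzzle that accepts BP_Paper actors and displays their decal materials.
; On overlap, a slot hides the paper at a far location, disables its collider, plays a timeline-driven insertion animation and shows the decal.
; With both animations flagged, a delayed check ejects both papers and resets the slots if slot 0's paper lacks Position 0.
; Slot 1's validity is never checked, and success has no action.
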(event OnComponentBeginOverlap(Collider0)
  (params (OverlappedComponent :type Primitive%20Component%20Object%20Reference) (OtherActor :type Actor%20Object%20Reference) (OtherComp :type Primitive%20Component%20Object%20Reference) (OtherBodyIndex :type Integer) (bFromSweep :type Boolean) (SweepResult :type Hit%20Result%20Structure%20%28by%20ref%29))
  (bind _decalarray (Variables|Default|GetDecalArray))
  (bind _output (Utilities|Array|Get(acopy) _decalarray))
  (bind _decal (Variables|/Script/Engine.DecalActor|GetDecal _output))
  (bind _asbp_paper (Utilities|Casting|CastToBP_Paper OtherActor))
  (Physics|SetSimulatePhysics (Variables|/Game/MyContent/GP/BPSantino/BP_Paper.BP_Paper_C|GetPaper _asbp_paper) false)
  (Transformation|SetActorLocation _asbp_paper "0.000000,0.000000,10000.000000" false false)
  (Rendering|SetVisibility _decal true false)
  (Rendering|Components|Decal|SetDecalMaterial _decal (Variables|/Game/MyContent/GP/BPSantino/BP_Paper.BP_Paper_C|GetDecalMat _asbp_paper))
  (Collision|SetCollisionEnabled (Variables|Default|GetCollider0) "NoCollision")
  (Variables|Default|SetPaper0 _asbp_paper)
  (if (== (Variables|/Game/MyContent/GP/BPSantino/BP_Paper.BP_Paper_C|GetPosition _asbp_paper) 0)
    (Variables|Default|SetIsPaper0Valide true))
  (Variables|Default|SetIsPaper0In true)
  (CallFunction|CEPaperAnim0)
  (if (and (Variables|Default|GetAnimIsOver0) (Variables|Default|GetAnimIsOver1))
    (Utilities|FlowControl|Delay 1.2)
    (CallFunction|CEVerif)))

(event OnComponentBeginOverlap(Collider1)
  (params (OverlappedComponent :type Primitive%20Component%20Object%20Reference) (OtherActor :type Actor%20Object%20Reference) (OtherComp :type Primitive%20Component%20Object%20Reference) (OtherBodyIndex :type Integer) (bFromSweep :type Boolean) (SweepResult :type Hit%20Result%20Structure%20%28by%20ref%29))
  (bind _decalarray (Variables|Default|GetDecalArray))
  (bind _output (Utilities|Array|Get(acopy) _decalarray 1))
  (bind _decal (Variables|/Script/Engine.DecalActor|GetDecal _output))
  (bind _asbp_paper (Utilities|Casting|CastToBP_Paper OtherActor))
  (Physics|SetSimulatePhysics (Variables|/Game/MyContent/GP/BPSantino/BP_Paper.BP_Paper_C|GetPaper _asbp_paper) false)
  (Transformation|SetActorLocation _asbp_paper "0.000000,0.000000,10000.000000" false false)
  (Rendering|SetVisibility _decal true false)
  (Rendering|Components|Decal|SetDecalMaterial _decal (Variables|/Game/MyContent/GP/BPSantino/BP_Paper.BP_Paper_C|GetDecalMat _asbp_paper))
  (Collision|SetCollisionEnabled (Variables|Default|GetCollider1) "NoCollision")
  (Variables|Default|SetPaper1 _asbp_paper)
  (if (== (Variables|/Game/MyContent/GP/BPSantino/BP_Paper.BP_Paper_C|GetPosition _asbp_paper) 0)
    (Variables|Default|SetIsPaper1Valide true))
  (Variables|Default|SetIsPaper1In true)
  (CallFunction|CEPaperAnim1)
  (if (and (Variables|Default|GetAnimIsOver0) (Variables|Default|GetAnimIsOver1))
    (Utilities|FlowControl|Delay 1.2)
    (CallFunction|CEVerif)))

(event Custom|CE_Verif
  (bind _paper0 (Variables|Default|GetPaper0))
  (bind _paper1 (Variables|Default|GetPaper1))
  (bind _decalarray (Variables|Default|GetDecalArray))
  (bind _output (Utilities|Array|Get(acopy) _decalarray))
  (bind _decal (Variables|/Script/Engine.DecalActor|GetDecal _output))
  (if (Variables|Default|GetIsPaper0In)
    (if (Variables|Default|GetIsPaper1In)
      (if (not (Variables|Default|GetIsPaper0Valide))
        (Rendering|SetVisibility (Variables|Default|GetPaperAnim0) false false)
        (Transformation|SetActorLocation _paper0 (Transformation|GetWorldLocation (Variables|Default|GetSphere0)) false true)
        (Physics|SetPhysicsLinearVelocity (Actor|GetComponentbyClass _paper0 "/Script/Engine.PrimitiveComponent") "0, 0, 0" false "None")
        (Physics|SetSimulatePhysics (Variables|/Game/MyContent/GP/BPSantino/BP_Paper.BP_Paper_C|GetPaper _paper0) true)
        (Transformation|SetActorLocation _paper1 (Transformation|GetWorldLocation (Variables|Default|GetSphere1)) false true)
        (Physics|SetPhysicsLinearVelocity (Actor|GetComponentbyClass _paper1 "/Script/Engine.PrimitiveComponent") "0, 0, 0" false "None")
        (Physics|SetSimulatePhysics (Variables|/Game/MyContent/GP/BPSantino/BP_Paper.BP_Paper_C|GetPaper _paper1) true)
        (Collision|SetCollisionEnabled (Variables|Default|GetCollider0) "QueryAndPhysics")
        (Collision|SetCollisionEnabled (Variables|Default|GetCollider1) "QueryAndPhysics")
        (Rendering|Components|Decal|SetDecalMaterial _decal 0)
        (Rendering|SetVisibility _decal false false)
        (Rendering|Components|Decal|SetDecalMaterial (Variables|/Script/Engine.DecalActor|GetDecal (Utilities|Array|Get(acopy) (Variables|Default|GetDecalArray) 1)) 0)
        (Variables|Default|SetIsPaper0Valide false)
        (Variables|Default|SetIsPaper1Valide false)
        (Variables|Default|SetIsPaper0In false)
        (Variables|Default|SetIsPaper1In false)))))

(event Custom|CE_PaperAnim1
  (bind _paperanim1 (Variables|Default|GetPaperAnim1))
  (bind _relativelocation (Variables|/Script/Engine.SceneComponent|GetRelativeLocation _paperanim1))
  (Rendering|Material|SetMaterial _paperanim1 0 "/Game/MyContent/GD/Mika/Materials/mat_paper.mat_paper")
  (Rendering|SetVisibility _paperanim1 true false)
  (bind _placement (Timeline|¨Placement PlayFromStart)
    (:Update
      (Transformation|SetRelativeLocation _paperanim1 (Math|Vector|MakeVector (.x _relativelocation) _placement (.z _relativelocation)) false false)
      (Variables|Default|SetAnimIsOver1 true))))

(event Custom|CE_PaperAnim0
  (bind _paperanim0 (Variables|Default|GetPaperAnim0))
  (bind _relativelocation (Variables|/Script/Engine.SceneComponent|GetRelativeLocation _paperanim0))
  (Rendering|Material|SetMaterial _paperanim0 0 "/Game/MyContent/GD/Mika/Materials/mat_paper.mat_paper")
  (Rendering|SetVisibility _paperanim0 true false)
  (bind _placement (Timeline|Placement PlayFromStart)
    (:Update
      (Transformation|SetRelativeLocation _paperanim0 (Math|Vector|MakeVector (.x _relativelocation) _placement (.z _relativelocation)) false false)
      (Variables|Default|SetAnimIsOver0 true))))

(fn ConstructionScript)