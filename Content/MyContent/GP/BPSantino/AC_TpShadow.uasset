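; AC_TpShadow is an actor component that teleports its owning BP_Character to the point the camera is aimed at.
; CE_GroundDetection line traces along the camera's forward vector with persistent debug drawing, storing the hit flag and impact coordinates.
; The stored Z adds the character's current world Z to the impact height.
; CE_Tp moves the character to the stored location only if the last trace hit.
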(event Custom|CE_GroundDetection
  (bind _asbp_character (Utilities|Casting|CastToBP_Character (Components|GetOwner)))
  (bind _output_get (Variables|Default|SetRefCharacter _asbp_character))
  (Variables|Default|SetStartLineTrace (Transformation|GetWorldLocation (Variables|/Game/MyContent/GP/Game/BP_Character.BP_Character_C|GetCamera _output_get)))
  (Variables|Default|SetEndLineTrace (+ (Transformation|GetWorldLocation (Variables|/Game/MyContent/GP/Game/BP_Character.BP_Character_C|GetCamera _output_get)) (* (Math|Vector|GetForwardVector (Variables|/Game/MyContent/GP/Game/BP_Character.BP_Character_C|GetCamera _output_get)) (Variables|Default|GetMultiplicateurLineTrace))))
  (bind (_outhit _returnvalue) (Collision|LineTraceByChannel (Variables|Default|GetStartLineTrace) (Variables|Default|GetEndLineTrace) "TraceTypeQuery4" false 0 "Persistent"))
  (if _returnvalue
    (Variables|Default|SetIsHit true)
    (else
      (Variables|Default|SetIsHit false)))
  (Variables|Default|SetImpact%20Point%20X (.x (.ImpactPoint (Collision|BreakHitResult _outhit))))
  (Variables|Default|SetImpact%20Point%20Y (.y (.ImpactPoint (Collision|BreakHitResult _outhit))))
  (Variables|Default|SetImpact%20Point%20Z (+ (.z (.ImpactPoint (Collision|BreakHitResult _outhit))) (.z (Transformation|GetActorLocation (Variables|Default|GetRefCharacter))))))

(event Custom|CE_Tp
  (if (Variables|Default|GetIsHit)
    (Transformation|SetActorLocation (Variables|Default|GetRefCharacter) (Math|Vector|MakeVector (Variables|Default|GetImpact%20Point%20X) (Variables|Default|GetImpact%20Point%20Y) (Variables|Default|GetImpact%20Point%20Z)) false false)))