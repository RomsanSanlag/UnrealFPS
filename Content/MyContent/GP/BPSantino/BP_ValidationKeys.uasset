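; BP_ValidationKeys is an actor that checks a key puzzle when something overlaps it.
; It loops through an array of keyholes and breaks out at the first one without the right key.
; On failure it ejects every locked key, then clears their locked flags after a short delay.
; The success branch only prints a placeholder message.
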(event Custom|CE_BreakLoop
  (bind _keyholesarray (Variables|Default|GetKeyHolesArray))
  (Utilities|Array|ForEachLoopwithBreak (Variables|Default|GetKeyHolesArray)) ; enters at Break
)

(event Collision|EventActorBeginOverlap
  (params (OtherActor :type Actor%20Object%20Reference))
  (bind _keyholesarray (Variables|Default|GetKeyHolesArray))
  (bind _array_element (Utilities|Array|ForEachLoopwithBreak (Variables|Default|GetKeyHolesArray))
    (:LoopBody
      (if (not (Variables|/Game/MyContent/GP/BPSantino/BP_KeyHole.BP_KeyHole_C|GetIsRightKey _array_element))
        (Variables|Default|SetIsBreak true)
        (CallFunction|CEBreakLoop)))
    (:Completed
      (if (Variables|Default|GetIsBreak)
        (for _array_element_2 _keyholesarray
          (if (Variables|/Game/MyContent/GP/BPSantino/BP_KeyHole.BP_KeyHole_C|GetIsKeyLocked _array_element_2)
            (Default|CEEjectKey _array_element_2)))
        (Utilities|FlowControl|Delay 0.3)
        (for _array_element_3 _keyholesarray
          (Variables|/Game/MyContent/GP/BPSantino/BP_KeyHole.BP_KeyHole_C|SetIsKeyLocked _array_element_3 false))
        (Variables|Default|SetIsBreak false)
        (Development|PrintString "done")
        (else
          (Development|PrintString "do something"))))))

(fn ConstructionScript)