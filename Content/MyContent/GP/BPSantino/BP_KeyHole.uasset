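; Keyhole actor that accepts a BP_Key entering its box and records whether the key's number matches its own.
; The inserted key stops simulating physics and teleports to a fixed location, while a proxy mesh copies its mesh and material for a timeline-driven insertion.
; CheckKey plays a turn animation on a locked key.
; CE_EjectKey restores physics, drops the key at the Sphere's location and resets the state and proxy.
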(event OnComponentBeginOverlap(Box)
  (params (OverlappedComponent :type Primitive%20Component%20Object%20Reference) (OtherActor :type Actor%20Object%20Reference) (OtherComp :type Primitive%20Component%20Object%20Reference) (OtherBodyIndex :type Integer) (bFromSweep :type Boolean) (SweepResult :type Hit%20Result%20Structure%20%28by%20ref%29))
  (if (not (Variables|Default|GetIsKeyLocked))
    (bind _asbp_key (Utilities|Casting|CastToBP_Key OtherActor))
    (Variables|Default|SetIsKeyLocked true)
    (bind _output_get (Variables|Default|SetBpKey _asbp_key))
    (Physics|SetSimulatePhysics (Variables|/Game/MyContent/GP/BPSantino/BP_Key.BP_Key_C|GetCube _output_get) false)
    (Transformation|SetActorLocation (Variables|Default|GetBpKey) "0.000000,0.000000,100.000000" false true)
    (Transformation|SetRelativeLocation (Variables|/Game/MyContent/GP/BPSantino/BP_Key.BP_Key_C|GetCube (Variables|Default|GetBpKey)) "0, 0, 0" false false)
    (if (== (Variables|/Game/MyContent/GP/BPSantino/BP_Key.BP_Key_C|GetKeyNumber (Variables|Default|GetBpKey)) (Variables|Default|GetKeyHoleNumber))
      (Development|PrintString "key lock and good")
      (Variables|Default|SetIsRightKey true)
      (else
        (Development|PrintString "key lock but not good")
        (Variables|Default|SetIsRightKey false)))
    (CallFunction|KeyAnimLock)
    ;[1 1 1] Sound_KeyInserted
    (bind _returnvalue (Audio|SpawnSound2D "/Game/MyContent/GD/Mika/Sounds/Sound_KeyLock_Cue.Sound_KeyLock_Cue" 1.0 1.0 0.0 0))
    (Audio|Components|Audio|SetVolumeMultiplier _returnvalue 0.75 :!class /Script/Engine.AudioComponent)))

(event Custom|CE_EjectKey
  (bind _bpkey (Variables|Default|GetBpKey))
  (bind _cube (Variables|/Game/MyContent/GP/BPSantino/BP_Key.BP_Key_C|GetCube _bpkey))
  (Physics|SetSimulatePhysics _cube true)
  (Transformation|SetActorLocation _bpkey (Transformation|GetWorldLocation (Variables|Default|GetSphere)) false true)
  (Physics|SetPhysicsLinearVelocity _cube "0, 0, 0" false "None")
  (Variables|Default|SetIsKeyLocked false)
  (Variables|Default|SetIsRightKey false)
  (CallFunction|ResetKeyAnim))

(event Custom|KeyAnimLock
  (bind _bpkey (Variables|Default|GetBpKey))
  (bind _keyanim (Variables|Default|GetKeyAnim))
  (bind _keyanim_2 (Variables|Default|GetKeyAnim))
  (bind _cube (Variables|/Game/MyContent/GP/BPSantino/BP_Key.BP_Key_C|GetCube _bpkey))
  (Components|StaticMesh|SetStaticMesh _keyanim (Variables|/Script/Engine.StaticMeshComponent|GetStaticMesh _cube))
  (Rendering|Material|SetMaterial _keyanim 0 (Rendering|Material|GetMaterial _cube 0))
  (Rendering|ToggleVisibility _keyanim_2 false)
  (bind _newtrack_0 (Timeline|Lock PlayFromStart)
    (:Update
      (Transformation|SetRelativeLocation _keyanim_2 (Math|Vector|MakeVector 0.0 0.0 _newtrack_0) false false))))

(event Custom|ResetKeyAnim
  (bind _keyanim (Variables|Default|GetKeyAnim))
  (Rendering|ToggleVisibility _keyanim false)
  (Transformation|SetRelativeRotation _keyanim (Math|Rotator|MakeRotator 0.0 0.0 -9e+01) false false))

(event Custom|CheckKey
  (if (Variables|Default|GetIsKeyLocked)
    (bind _check (Timeline|Check PlayFromStart)
      (:Update
        (Transformation|SetRelativeRotation (Variables|Default|GetKeyAnim) (Math|Rotator|MakeRotator 0.0 0.0 _check) false false)))))

(fn ConstructionScript)