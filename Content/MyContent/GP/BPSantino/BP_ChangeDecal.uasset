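; BP_ChangeDecal is a Blueprint that swaps what is visible in the scene, replacing four referenced panels with a text object.
; The Switch event hides the root components of Panel0 to Panel3 and shows the root of Text, without propagating to child components.
; A second event, CustomEvent, runs the same logic; the swap is one-way and the construction script is empty.
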(event Custom|CustomEvent
  (Rendering|SetVisibility (Variables|/Script/Engine.Actor|GetRootComponent (Variables|Default|GetPanel_0)) false false)
  (Rendering|SetVisibility (Variables|/Script/Engine.Actor|GetRootComponent (Variables|Default|Gettext)) true false))

(event EventSwitch
  (Rendering|SetVisibility (Variables|/Script/Engine.Actor|GetRootComponent (Variables|Default|GetPanel_0)) false false)
  (Rendering|SetVisibility (Variables|/Script/Engine.Actor|GetRootComponent (Variables|Default|Gettext)) true false))

(fn ConstructionScript)