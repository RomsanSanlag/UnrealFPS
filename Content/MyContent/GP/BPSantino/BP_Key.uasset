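; BP_Key is a puzzle key that reports whether it sits in the key hole with the matching number.
; When its Cube overlaps a BP_KeyHole, it caches that hole, sets IsKeyLocked and calls CEValideKey or CEKeyNotValid depending on whether KeyHoleNumber equals KeyNumber.
; Any actor end overlap invalidates the cached hole if the numbers match, without checking the other actor, and also sets IsKeyLocked true.
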(event OnComponentBeginOverlap(Cube)
  (params (OverlappedComponent :type Primitive%20Component%20Object%20Reference) (OtherActor :type Actor%20Object%20Reference) (OtherComp :type Primitive%20Component%20Object%20Reference) (OtherBodyIndex :type Integer) (bFromSweep :type Boolean) (SweepResult :type Hit%20Result%20Structure%20%28by%20ref%29))
  (bind _asbp_key_hole (Utilities|Casting|CastToBP_KeyHole OtherActor))
  (bind _output_get (Variables|Default|SetAs%20BP%20Key%20Hole _asbp_key_hole))
  (Variables|Default|SetIsKeyLocked true)
  (if (== (Variables|/Game/MyContent/GP/BPSantino/BP_KeyHole.BP_KeyHole_C|GetKeyHoleNumber _output_get) (Variables|Default|GetKeyNumber))
    (Development|PrintString "key lock and good")
    (Default|CEValideKey (Variables|Default|GetAs%20BP%20Key%20Hole))
    (else
      (Development|PrintString "key lock but not good")
      (Default|CEKeyNotValid (Variables|Default|GetAs%20BP%20Key%20Hole)))))

(event Collision|EventActorEndOverlap
  (params (OtherActor :type Actor%20Object%20Reference))
  (Variables|Default|SetIsKeyLocked true)
  (if (== (Variables|/Game/MyContent/GP/BPSantino/BP_KeyHole.BP_KeyHole_C|GetKeyHoleNumber (stale OnComponentBeginOverlap(Cube) _output_get)) (Variables|Default|GetKeyNumber))
    (Default|CEKeyNotValid (Variables|Default|GetAs%20BP%20Key%20Hole))))

(fn ConstructionScript)