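; BP_End is an end-zone actor that shows a finish screen when the player character enters its DeathZone trigger.
; The overlap event checks for a BP_Character with the Player tag, then calls the end event.
; That event creates a fresh W_FinishScreen, adds it to the viewport and plays its screen animation, ending on a delay with nothing after it.
; The widget created at BeginPlay is never displayed, only removed.
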(event OnComponentBeginOverlap(DeathZone)
  (params (OverlappedComponent :type Primitive%20Component%20Object%20Reference) (OtherActor :type Actor%20Object%20Reference) (OtherComp :type Primitive%20Component%20Object%20Reference) (OtherBodyIndex :type Integer) (bFromSweep :type Boolean) (SweepResult :type Hit%20Result%20Structure%20%28by%20ref%29))
  ;[1 1 1] Detect Player in zone
  (Utilities|Casting|CastToBP_Character OtherActor)
  (if (Actor|ActorHasTag OtherActor "Player")
    (CallFunction|CEEnd)))

(event Custom|CE_End
  ;[1 1 1] Black screen
  (Widget|RemovefromParent (Variables|Default|GetW_EndScreen))
  (bind _returnvalue (UserInterface|CreateWidget "/Game/MyContent/GP/UMG/W_FinishScreen.W_FinishScreen_C"))
  (UserInterface|Viewport|AddtoViewport _returnvalue 0)
  (UserInterface|Animation|PlayAnimation _returnvalue (Variables|/Game/MyContent/GP/UMG/W_FinishScreen.W_FinishScreen_C|GetScreenAnimation _returnvalue) 0.0 1 "Forward" 1.0 false)
  (Utilities|FlowControl|Delay 2.0))

(event EventBeginPlay
  ;[1 1 1] Generate black Screen
  (bind _returnvalue (UserInterface|CreateWidget "/Game/MyContent/GP/UMG/W_FinishScreen.W_FinishScreen_C"))
  (Variables|Default|SetW_EndScreen _returnvalue))

(fn ConstructionScript)