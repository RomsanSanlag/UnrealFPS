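; BP_Death is a death zone that respawns the player character when it overlaps the DeathZone component.
; On death it releases the character's PhysicsHandle, plays the W_DeathScreen animation and, after a short delay, teleports the character to a respawn location.
; The Switch event permanently changes the destination from RespawnLocationIn to RespawnLocationOut.
; All top-level death screen widgets are then removed from the viewport.
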(event OnComponentBeginOverlap(DeathZone)
  (params (OverlappedComponent :type Primitive%20Component%20Object%20Reference) (OtherActor :type Actor%20Object%20Reference) (OtherComp :type Primitive%20Component%20Object%20Reference) (OtherBodyIndex :type Integer) (bFromSweep :type Boolean) (SweepResult :type Hit%20Result%20Structure%20%28by%20ref%29))
  ;[1 1 1] Detect Player in zone
  (Utilities|Casting|CastToBP_Character OtherActor)
  (CallFunction|CEDeath))

(event Custom|CE_Death
  (bind _as_bp_character (Variables|Default|GetAs%20BP%20Character))
  ;[1 1 1] Black screen
  (Physics|Components|PhysicsHandle|ReleaseComponent (Variables|/Game/MyContent/GP/Game/BP_Character.BP_Character_C|GetPhysicsHandle (Variables|Default|GetAs%20BP%20Character)))
  (bind _returnvalue (UserInterface|CreateWidget "/Game/MyContent/GP/UMG/W_DeathScreen.W_DeathScreen_C"))
  (UserInterface|Viewport|AddtoViewport _returnvalue 0)
  (UserInterface|Animation|PlayAnimation _returnvalue (Variables|/Game/MyContent/GP/UMG/W_DeathScreen.W_DeathScreen_C|GetScreenAnimation _returnvalue) 0.0 1 "Forward" 1.0 false)
  (Utilities|FlowControl|Delay 2.0)
  (if (Variables|Default|GetSwitchRespawn)
    (Transformation|SetActorLocation _as_bp_character (Transformation|GetActorLocation (Variables|Default|GetRespawn%20Location%20Out)) false true)
    (else
      (Transformation|SetActorLocation _as_bp_character (Transformation|GetActorLocation (Variables|Default|GetRespawn%20Location%20In)) false true)))
  (bind _foundwidgets (Widget|GetAllWidgetsOfClass "/Game/MyContent/GP/UMG/W_DeathScreen.W_DeathScreen_C" true))
  (Widget|RemovefromParent _foundwidgets))

(event EventBeginPlay
  ;[1 1 1] Generate black Screen
  (bind _returnvalue (UserInterface|CreateWidget "/Game/MyContent/GP/UMG/W_DeathScreen.W_DeathScreen_C"))
  (Variables|Default|SetW_blackScreen _returnvalue)
  (bind _asbp_character (Utilities|Casting|CastToBP_Character (Game|GetPlayerCharacter 0)))
  (Variables|Default|SetAs%20BP%20Character _asbp_character))

(event EventSwitch
  ;[1 1 1] Black screen
  (Variables|Default|SetSwitchRespawn true))

(fn ConstructionScript)