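; BP_Respawn is a waypoint actor that records a respawn location; the respawn itself is not handled here.
; When BP_Character overlaps the WayPoint component and the game mode is GM_Game, it stores the character's position in RespawnLocation and spawns a decal there.
; A hit on WayPoint stores the actor's own location instead, without any cast checks.
; Both paths print debug strings.
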(event OnComponentBeginOverlap(WayPoint)
  (params (OverlappedComponent :type Primitive%20Component%20Object%20Reference) (OtherActor :type Actor%20Object%20Reference) (OtherComp :type Primitive%20Component%20Object%20Reference) (OtherBodyIndex :type Integer) (bFromSweep :type Boolean) (SweepResult :type Hit%20Result%20Structure%20%28by%20ref%29))
  ;[1 0.01578 0] Comment
  (Utilities|Casting|CastToBP_Character OtherActor)
  (Utilities|Casting|CastToGM_Game (Game|GetGameMode))
  (Development|PrintString "Hello")
  (bind _output_get (Variables|Default|SetRespawnLocation (Transformation|GetActorLocation (Variables|Default|GetCharacter))))
  (Rendering|Decal|SpawnDecalatLocation 0 "0, 0, 0" _output_get "-90.000000,0.000000,0.000000" 0.0)
  (Development|PrintString "waypoint"))

(event OnComponentHit(WayPoint)
  (params (HitComponent :type Primitive%20Component%20Object%20Reference) (OtherActor :type Actor%20Object%20Reference) (OtherComp :type Primitive%20Component%20Object%20Reference) (NormalImpulse :type Vector :default "0, 0, 0") (Hit :type Hit%20Result%20Structure%20%28by%20ref%29))
  (Variables|Default|SetRespawnLocation (Transformation|GetActorLocation))
  (Development|PrintString "Touch Waypoint"))

(event EventBeginPlay)

(event EventTick
  (params (DeltaSeconds :type Float%20%28single-precision%29)))

(fn ConstructionScript)