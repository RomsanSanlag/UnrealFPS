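; BP_GameManager is a game manager actor that handles player death and respawn through a death zone.
; When a character hits the DeathZone component, a death event teleports the character to the respawn point's stored location.
; It then prints a failure message and calls the character's respawn event through the respawn reference.
; A damage event exists but is empty.
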(event OnComponentHit(DeathZone)
  (params (HitComponent :type Primitive%20Component%20Object%20Reference) (OtherActor :type Actor%20Object%20Reference) (OtherComp :type Primitive%20Component%20Object%20Reference) (NormalImpulse :type Vector :default "0, 0, 0") (Hit :type Hit%20Result%20Structure%20%28by%20ref%29))
  (Utilities|Casting|CastToBP_Character OtherActor)
  (CallFunction|CEDeath))

(event Custom|CE_Death
  (Transformation|SetActorLocation (Variables|Default|GetBP_Character) (Variables|/Game/MyContent/GP/BPLeo/BP_Respawn.BP_Respawn_C|GetRespawnLocation (Variables|Default|GetBP_Respawn)) false true)
  (Development|PrintText "FAILED!")
  (Default|CERespawn (Variables|/Game/MyContent/GP/BPLeo/BP_Respawn.BP_Respawn_C|GetCharacter (Variables|Default|GetBP_Respawn))))

(event Custom|CE_DealDamages)

(event EventBeginPlay)

(event Collision|EventActorBeginOverlap
  (params (OtherActor :type Actor%20Object%20Reference)))

(event EventTick
  (params (DeltaSeconds :type Float%20%28single-precision%29)))

(fn ConstructionScript)