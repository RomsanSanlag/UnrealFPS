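; Player character Blueprint that respawns the player after the character is destroyed.
; BeginPlay runs the respawn setup, which checks that player 0 is a BP_Character and binds a handler to OnDestroyed.
; After a short delay, that handler spawns a new BP_Character at the BPRespawn transform, has the player controller possess it and calls the respawn event again, with debug prints along the way.
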(event Custom|CE_OnDestroy
  (params (DestroyedActor :type Actor%20Object%20Reference))
  ;[1 0.008162 0] aaaaahhhhhhhhh
  (Utilities|FlowControl|Delay 2.0)
  (bind _returnvalue (Game|SpawnActorfromClass "BP_Character_C" (Variables|/Game/MyContent/GP/BPLeo/BP_Respawn.BP_Respawn_C|GetSpawnTransform (Variables|Default|GetBP_respawn)) "Undefined" 0 0))
  (Pawn|Possess (Game|GetPlayerController 0) _returnvalue)
  (CallFunction|CERespawn)
  (Development|PrintString "spawn"))

(event Custom|CE_Respawn
  (Utilities|Casting|CastToBP_Character (Game|GetPlayerCharacter 0))
  (Development|PrintString "Spawn")
  (Game|BindEventtoOnDestroyed (delegate Custom|CE_OnDestroy)))

(event EventBeginPlay
  (Utilities|Casting|CastToBP_Character (Game|GetPlayerCharacter 0))
  (Development|PrintString "Spawn")
  (Game|BindEventtoOnDestroyed (delegate Custom|CE_OnDestroy)))

(event Collision|EventActorBeginOverlap
  (params (OtherActor :type Actor%20Object%20Reference)))

(event EventTick
  (params (DeltaSeconds :type Float%20%28single-precision%29)))

(fn ConstructionScript)