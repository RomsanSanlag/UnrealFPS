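; BP_PassageSecret is a secret passage door in the labyrinth that opens once two conditions are met.
; TorchOn and ZoneOn events each set a flag, both reset at BeginPlay, then call Open.
; When both flags are true, Open prints a message and instantly moves the actor 500 units up, with no animation or guard against repeat calls.
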(event Custom|Open
  ;[1 1 1] TryOpen
  (if (Variables|Default|GetZone)
    (if (Variables|Default|GetToch)
      (Development|PrintString "Door is Opened!")
      (Transformation|SetActorLocation (+ (Transformation|GetActorLocation) "0.000000,0.000000,500.000000") false false))))

(event Custom|ZoneOn
  ;[1 1 1] ConditionZoneOnAndTryOpenDoor
  (Variables|Default|SetZone true)
  (CallFunction|Open))

(event Custom|TorchOn
  ;[1 1 1] ConditionTorchOnAndTryOpenDoor
  (Variables|Default|SetToch true)
  (CallFunction|Open))

(event EventBeginPlay
  ;[1 1 1] ResetConditions
  (Variables|Default|SetToch false)
  (Variables|Default|SetZone false))

(fn ConstructionScript)